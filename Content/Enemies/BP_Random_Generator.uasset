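; Enemy spawner for the space shooter that creates enemies on a looping timer.
; Each tick picks BP_EnemyBase or BP_EnemyVariant randomly within the game mode's Level, clamped by MaxNumEnemies, and spawns it at a random component tagged SpawnPoint.
; Each spawned enemy's destroy event lowers SpawnTime, but the timer is set only at BeginPlay, so its interval stays unchanged.
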(event Custom|Spawn
  (bind _enemyspawned (CallFunction|SpawnEnemy))
  (Utilities|Casting|CastToBP_EnemyBase _enemyspawned)
  (EventDispatchers|BindEventtoOnenemyDestroy (delegate Custom|EnemyDestroyed)))

(event Custom|EnemyDestroyed
  (Variables|Default|SetSpawnTime (- (Variables|Default|GetSpawnTime) 1.0)))

(event EventBeginPlay
  (Utilities|Time|SetTimerbyEvent (delegate Custom|Spawn) (Variables|Default|GetSpawnTime) true)
  (bind _asbp_space_shooter_gamemode (Utilities|Casting|CastToBP_Space_Shooter_Gamemode (Game|GetGameMode)))
  (Variables|Default|Setm_GameMode _asbp_space_shooter_gamemode))

(event Collision|EventActorBeginOverlap
  (params (OtherActor :type Actor%20Object%20Reference)))

(event EventTick
  (params (DeltaSeconds :type Float%20%28single-precision%29)))

(fn ConstructionScript)

(fn SpawnEnemy
  (bind _returnvalue (Actor|GetComponentsbyTag "/Script/Engine.SceneComponent" "SpawnPoint"))
  (bind _newparam (CallFunction|GetClasstoSpawn (Math|Random|RandomInteger (Variables|/Game/BP_Space_Shooter_Gamemode.BP_Space_Shooter_Gamemode_C|GetLevel (Variables|Default|Getm_GameMode)))))
  (bind _asscene_component (Utilities|Casting|CastToSceneComponent (Utilities|Array|Get(acopy) _returnvalue (Math|Random|RandomInteger (Utilities|Array|Length _returnvalue)))))
  (bind _returnvalue_2 (Game|SpawnActorfromClass _newparam (Transformation|GetWorldTransform _asscene_component) "AdjustIfPossibleButAlwaysSpawn" "MultiplyWithRoot" 0 0))
  (bind _asbp_enemy_base (Utilities|Casting|CastToBP_EnemyBase _returnvalue_2))
  (return _asbp_enemy_base))

(fn GetClasstoSpawn
  (params (Type :type Integer))
  (return (Utilities|Select :Index (Math|Integer|Clamp(Integer) Type 0 (- (Variables|Default|GetMaxNumEnemies) 1)) :Option%200 "/Game/Enemies/BP_EnemyBase.BP_EnemyBase_C" :Option%201 "/Game/Enemies/BP_EnemyVariant.BP_EnemyVariant_C")))